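; TestingCharacter is a test pawn that moves with standard look and move axes and can try out teleporting from the keyboard.
; On BeginPlay it offsets VRRoot upward and lets the camera follow control rotation, so movement follows the camera's forward and right vectors.
; Holding Space calls ScanToTeleport from the camera, and releasing it calls StopTryingToTeleport, neither defined here.
; Tick writes the current frame rate to a TextRender.
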(event `self.ReceiveBeginPlay`
  (`SceneComponent.K2_SetRelativeLocation` (`self.VRRoot`) (0.0 0.0 50.0) false false)
  (set `CameraComponent.bUsePawnControlRotation` true (`self.Camera`)))

(event `InputAxis|LookUp`
  (params (AxisValue :type "Float (single-precision)"))
  (`self.AddControllerPitchInput` AxisValue))

(event `InputAxis|LookRight`
  (params (AxisValue :type "Float (single-precision)"))
  (`self.AddControllerYawInput` AxisValue))

(event `Key|SpaceBar`
  (params (Key :type "Key Structure"))
  (:`Pressed`
    (`self.ScanToTeleport` (`self.Camera`)))
  (:`Released`
    (`self.StopTryingToTeleport`)))

(event `InputAxis|MoveForward`
  (params (AxisValue :type "Float (single-precision)"))
  (`self.AddMovementInput` (`SceneComponent.GetForwardVector` (`self.Camera`)) AxisValue))

(event `InputAxis|MoveRight`
  (params (AxisValue :type "Float (single-precision)"))
  (`self.AddMovementInput` (`SceneComponent.GetRightVector` (`self.Camera`)) AxisValue))

(event `self.ReceiveTick`
  (params (DeltaSeconds :type "Float (single-precision)"))
  (`TextRenderComponent.K2_SetText` (`self.TextRender`) (`KismetTextLibrary.Conv_DoubleToText` (/ 1.0 DeltaSeconds) "HalfToEven")))

(fn `UserConstructionScript`)