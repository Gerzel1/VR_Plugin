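; BP_HighlightMesh is a component that builds a highlight around its owning actor from duplicate meshes.
; It caches the owner's static mesh components on BeginPlay.
; CreateMesh runs once, spawning a slightly enlarged, shadowless StaticMeshActor at each component's transform with every slot set to OutLineMaterial.
; The copies are stored in CurrentMeshes but not attached to the owner, and DestroyMeshes is an empty stub.
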(event `self.ReceiveBeginPlay`
  (set `self.AllMeshes` (`Actor.K2_GetComponentsByClass` (`self.GetOwner`) "/Script/Engine.StaticMeshComponent")))

(event `CreateMesh`
  (if (not (`self.CreatedMeshes`))
    (for _array_element (`self.AllMeshes`)
      (bind (_returnvalue_location _returnvalue_rotation _returnvalue_scale) (`KismetMathLibrary.BreakTransform` (`SceneComponent.K2_GetComponentToWorld` _array_element)))
      (bind _returnvalue (`|SpawnActorFromClass` "/Script/Engine.StaticMeshActor" (`KismetMathLibrary.MakeTransform` _returnvalue_location _returnvalue_rotation (* _returnvalue_scale 1.05)) "AlwaysSpawn" "OverrideRootScale" null null))
      (bind _staticmeshcomponent (`StaticMeshActor.StaticMeshComponent` _returnvalue))
      (`SceneComponent.SetMobility` _staticmeshcomponent "Movable")
      (`StaticMeshComponent.SetStaticMesh` _staticmeshcomponent (`StaticMeshComponent.StaticMesh` _array_element))
      (`PrimitiveComponent.SetCastShadow` _staticmeshcomponent false)
      (`KismetArrayLibrary.Array_Add` (`self.CurrentMeshes`) _returnvalue)
      (for (_ _array_index) (`MeshComponent.GetMaterials` _staticmeshcomponent)
        (`PrimitiveComponent.SetMaterial` _staticmeshcomponent _array_index "/Gerzel_VR/OutLineMaterial.OutLineMaterial")))
    (set `self.CreatedMeshes` true)))

(event `DestroyMeshes`)